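; Player controller for the Statue game that sets up input and UI, then forwards player actions to the possessed StatuePlayer pawn.
; On possess it adds the IMC_Actions Enhanced Input mapping context, shows a WBP_Counter widget and caches the pawn as a StatuePlayer.
; Move and Look input pass their values straight to that pawn, while Shoot calls its ShootMessage function on press.
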(event Input|EnhancedActionEvents|EnhancedInputActionMove
  (params (ActionValue :type Vector%202D%20Structure) (ElapsedSeconds :type Float%20%28double-precision%29) (TriggeredSeconds :type Float%20%28double-precision%29) (InputAction :type Input%20Action%20Object%20Reference :default "/Game/Actions/Move.Move"))
  (:Triggered
    (Class|StatuePlayer|Move (Variables|Default|GetStatuePlayer) ActionValue)))

(event Input|EnhancedActionEvents|EnhancedInputActionLook
  (params (ActionValue :type Vector%202D%20Structure) (ElapsedSeconds :type Float%20%28double-precision%29) (TriggeredSeconds :type Float%20%28double-precision%29) (InputAction :type Input%20Action%20Object%20Reference :default "/Game/Actions/Look.Look"))
  (:Triggered
    (Class|StatuePlayer|Look (Variables|Default|GetStatuePlayer) ActionValue)))

(event Input|EnhancedActionEvents|EnhancedInputActionShoot
  (params (ActionValue :type Boolean) (ElapsedSeconds :type Float%20%28double-precision%29) (TriggeredSeconds :type Float%20%28double-precision%29) (InputAction :type Input%20Action%20Object%20Reference :default "/Game/Actions/Shoot.Shoot"))
  (:Started
    (Class|ShootInterface|Shoot(Message) (Variables|Default|GetStatuePlayer))))

(event EventPossess
  (params (PossessedPawn :type Pawn%20Object%20Reference))
  (Input|AddMappingContext (PlayerController|LocalPlayerSubsystems|GetEnhancedInputLocalPlayerSubsystem) "/Game/Actions/IMC_Actions.IMC_Actions" 0 "(bIgnoreAllPressedKeysUntilRelease=True,bForceImmediately=False)")
  (bind _returnvalue (UserInterface|CreateWidget "/Game/Statue/WBP_Counter.WBP_Counter_C" self))
  (UserInterface|Viewport|AddtoViewport _returnvalue 0)
  (bind _asstatue_player (Utilities|Casting|CastToStatuePlayer PossessedPawn))
  (Variables|Default|SetStatuePlayer _asstatue_player))

(fn ConstructionScript)