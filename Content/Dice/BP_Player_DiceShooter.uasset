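; BP_Player_DiceShooter is a player Blueprint that shoots physics dice from the camera.
; Its Shoot event spawns a BP_Die a short distance ahead of the camera with a random rotation and the camera's scale.
; It then launches the die's static mesh with a strong, mass-dependent impulse along the camera's forward vector.
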(event EventShoot
  (bind _cameracomponent (Variables|Default|GetCameraComponent))
  (bind _returnvalue (Transformation|GetWorldTransform _cameracomponent))
  (bind _returnvalue_2 (Math|Vector|GetForwardVector _cameracomponent))
  (bind _returnvalue_3 (Game|SpawnActorfromClass "/Game/Dice/BP_Die.BP_Die_C" (Math|Transform|MakeTransform (+ (.location _returnvalue) (* _returnvalue_2 1e+02)) (Math|Random|RandomRotator false) (.scale _returnvalue)) "Undefined" "MultiplyWithRoot" 0 0))
  (Physics|AddImpulse (Variables|/Script/Forsbergs.Die|GetStaticMeshComponent _returnvalue_3) (* _returnvalue_2 1e+05) "None" false))

(fn ConstructionScript)